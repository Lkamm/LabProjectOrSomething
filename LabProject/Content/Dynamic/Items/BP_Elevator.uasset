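; BP_Elevator is an actor that moves vertically between its starting height and a point 45 units above it.
; The rise event uses a FlipFlop to play or reverse a Timeline that lerps the actor's Z location.
; Each completed move switches the point light between red and green.
; Overlap events set CanToggleSwitch on BP_FirstPersonCharacter while it is within the elevator's overlap area.
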(event `self.ReceiveTick`
  (params (DeltaSeconds :type "Float (single-precision)")))

(event `rise`
  (bind (_returnvalue_x _returnvalue_y) (`KismetMathLibrary.BreakVector` (`self.K2_GetActorLocation`)))
  (`/Engine/EditorBlueprintResources/StandardMacros.FlipFlop`
    (:`A`
      (bind (_direction _newtrack_1) (`Timeline|Timeline` :`NewTime` (stale `self.ReceiveTick` DeltaSeconds) :!label _label)
        (:`Update`
          (`self.K2_SetActorLocation` (`KismetMathLibrary.MakeVector` _returnvalue_x _returnvalue_y (`KismetMathLibrary.Lerp` (`self.start`) (`self.end`) _newtrack_1))))
        (:`Finished`
          (if (`self.wasPosA?`)
            (`LightComponent.SetLightColor` (`self.PointLight`) (make `LinearColor` 225.0 0.0 0.0 1.0) true)
            (set `self.wasPosA?` false)
            (else
              (`LightComponent.SetLightColor` (`self.PointLight`) (make `LinearColor` 0.0 225.0 0.0 1.0) true)
              (set `self.wasPosA?` true))))))
    (:`B`
      (goto _label :!via `Reverse`))))

(event `self.ReceiveBeginPlay`
  (bind (_returnvalue_x _returnvalue_y _returnvalue_z) (`KismetMathLibrary.BreakVector` (`self.K2_GetActorLocation`)))
  (set `self.start` _returnvalue_z)
  (set `self.end` (+ _returnvalue_z 45.0))
  (set `self.wasPosA?` true))

(event `self.ReceiveActorEndOverlap`
  (params (OtherActor :type "Actor Object Reference"))
  (bind _asbp_first_person_character (cast `/Game/Dynamic/FirstPerson/Blueprints/BP_FirstPersonCharacter` OtherActor))
  (set `/Game/Dynamic/FirstPerson/Blueprints/BP_FirstPersonCharacter.canToggleSwitch?` false _asbp_first_person_character))

(event `self.ReceiveActorBeginOverlap`
  (params (OtherActor :type "Actor Object Reference"))
  (bind _asbp_first_person_character (cast `/Game/Dynamic/FirstPerson/Blueprints/BP_FirstPersonCharacter` OtherActor))
  (set `/Game/Dynamic/FirstPerson/Blueprints/BP_FirstPersonCharacter.canToggleSwitch?` true _asbp_first_person_character))

(fn `UserConstructionScript`)